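; BP_SwingHoop is a trigger actor that pushes a referenced BP_Swing when something overlaps its Sphere.
; On begin overlap it casts ActorRef to BP_Swing and adds a velocity-change impulse to SwingSphere, built from per-axis impulse variables.
; The Steppingon flag blocks repeat impulses until an end overlap clears it.
; The overlapping actor is not filtered.
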(event OnComponentEndOverlap(Sphere)
  (params (OtherActor :type Actor%20Object%20Reference) (OtherComp :type Primitive%20Component%20Object%20Reference) (OtherBodyIndex :type Integer))
  (Variables|Default|Setsteppingon false))

(event OnComponentBeginOverlap(Sphere)
  (params (OtherActor :type Actor%20Object%20Reference) (OtherComp :type Primitive%20Component%20Object%20Reference) (OtherBodyIndex :type Integer) (bFromSweep :type Boolean) (SweepResult :type Hit%20Result%20Structure%20%28by%20ref%29))
  (if (not (Variables|Default|Getsteppingon))
    (Variables|Default|Setsteppingon true)
    (bind _asbp_swing (Utilities|Casting|CastToBP_Swing (Variables|Default|Getactor_ref)))
    (Physics|AddImpulse (Variables|/Game/Blueprints/BP_Swing.BP_Swing_C|GetSwingSphere _asbp_swing) (Math|Vector|MakeVector (Variables|Default|Getximpulse) (Variables|Default|Getyimpulse) (Variables|Default|Getzimpulse)) "None" true)))

(event EventBeginPlay)

(event EventActorBeginOverlap
  (params (OtherActor :type Actor%20Object%20Reference)))

(event EventTick
  (params (DeltaSeconds :type Float%20%28single-precision%29)))

(fn ConstructionScript)