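; BP_Greeting is a Blueprint that shows a greeting as three text render components (top text, main text and subtext) with controllable opacity.
; On BeginPlay it creates and stores a dynamic material instance for each text component.
; The OpacitywithValue event pushes a given value into the Opacity scalar parameter of all three instances, so the text can be faded together from outside.
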(event EventBeginPlay
  (Utilities|FlowControl|Sequence
    (:then_0
      (bind _returnvalue (Rendering|Material|CreateDynamicMaterialInstance (Variables|Default|GetTextRender) 0 0 :!class /Script/Engine.PrimitiveComponent))
      (Variables|Default|SetTextRenderDMI _returnvalue))
    (:then_1
      (bind _returnvalue_2 (Rendering|Material|CreateDynamicMaterialInstance (Variables|Default|GetSubtextRender1) 0 0 :!class /Script/Engine.PrimitiveComponent))
      (Variables|Default|SetSubtextRenderDMI _returnvalue_2))
    (:then_2
      (bind _returnvalue_3 (Rendering|Material|CreateDynamicMaterialInstance (Variables|Default|GetTopTextRender) 0 0 :!class /Script/Engine.PrimitiveComponent))
      (Variables|Default|SetToptextRenderDMI_0 _returnvalue_3))))

(event EventOpacitywithValue
  (params (Value :type Float%20%28single-precision%29))
  (Utilities|FlowControl|Sequence
    (:then_0
      (Rendering|Material|SetScalarParameterValue (Variables|Default|GetTextRenderDMI) "Opacity" Value :!class /Script/Engine.MaterialInstanceDynamic))
    (:then_1
      (Rendering|Material|SetScalarParameterValue (Variables|Default|GetSubtextRenderDMI) "Opacity" Value :!class /Script/Engine.MaterialInstanceDynamic))
    (:then_2
      (Rendering|Material|SetScalarParameterValue (Variables|Default|GetToptextRenderDMI_0) "Opacity" Value :!class /Script/Engine.MaterialInstanceDynamic))))

(fn ConstructionScript)